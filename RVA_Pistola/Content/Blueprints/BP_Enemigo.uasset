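; BP_Enemigo is an enemy actor that turns into a randomized primitive shape and is launched upward when play begins.
; BeginPlay selects the static mesh at random, though RandomInteger(2) only yields Cylinder or Cone, never the wired Cube.
; It then applies a random rotation and uniform scale, and adds a random Z impulse to the mesh.
; Overlap, Tick and the construction script are empty.
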(event EventBeginPlay
  (Components|StaticMesh|SetStaticMesh (Variables|Default|GetStaticMesh) (Utilities|Select :Index (Math|Random|RandomInteger 2) :Option%200 "/Engine/BasicShapes/Cylinder.Cylinder" :Option%201 "/Engine/BasicShapes/Cone.Cone" :Option%202 "/Engine/BasicShapes/Cube.Cube"))
  (Transformation|SetRelativeTransform (Variables|Default|GetStaticMesh) (Math|Transform|MakeTransform (Variables|/Script/Engine.SceneComponent|GetRelativeLocation (Variables|Default|GetStaticMesh)) (Math|Random|RandomRotator false) (Math|Conversions|ToVector(Float) (Math|Random|RandomFloatinRange 1.0 3.0))) false false)
  (Physics|AddImpulse (Variables|Default|GetStaticMesh) (Math|Vector|MakeVector 0.0 0.0 (Math|Random|RandomFloatinRange 1.5e+05 3e+05)) "None" false))

(event Collision|EventActorBeginOverlap
  (params (OtherActor :type Actor%20Object%20Reference)))

(event EventTick
  (params (DeltaSeconds :type Float%20%28single-precision%29)))

(fn ConstructionScript)