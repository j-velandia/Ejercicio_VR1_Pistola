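; VR player Blueprint that handles gun pickup, shooting, reloading and kill counting.
; On the first left-hand overlap with a BP_Gun, it destroys that gun, spawns a new one attached to the left motion controller and hides the hand.
; Enhanced Input drives shooting and reloading once armed.
; These actions, pickup and AddKill refresh bullets, kills and notifications on a HUD widget, cached from an in-world widget actor one second after BeginPlay.
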(event OnComponentBeginOverlap(LeftHand)
  (params (OverlappedComponent :type Primitive%20Component%20Object%20Reference) (OtherActor :type Actor%20Object%20Reference) (OtherComp :type Primitive%20Component%20Object%20Reference) (OtherBodyIndex :type Integer) (bFromSweep :type Boolean) (SweepResult :type Hit%20Result%20Structure%20%28by%20ref%29))
  (bind _hudreference (Variables|Default|GetHUDReference))
  (bind _asbp_gun (Utilities|Casting|CastToBP_Gun OtherActor))
  (Utilities|FlowControl|DoOnce false
    (:Completed
      (Actor|DestroyActor _asbp_gun)
      (Development|SetHiddeninGame (Variables|Default|GetLeftHand) false false)
      (bind _returnvalue (Game|SpawnActorfromClass "/Game/Blueprints/BP_Gun.BP_Gun_C" (Transformation|GetWorldTransform (Variables|Default|GetLeftMotionController)) "Undefined" "MultiplyWithRoot" 0 0))
      (bind _output_get (Variables|Default|SetGun _returnvalue))
      (Transformation|AttachComponentToComponent _output_get (Variables|Default|GetLeftMotionController) "None" "SnapToTarget" "SnapToTarget" "SnapToTarget" true)
      (Rendering|SetVisibility (Variables|Default|GetLeftHand) false false)
      (Variables|Default|SetisArmed true)
      (Default|ShowDetailPanel _hudreference)
      (Default|UpdateHUD _hudreference (Variables|/Game/Blueprints/BP_Gun.BP_Gun_C|GetcurrentBullets (Variables|Default|GetGun)) (Variables|Default|Getkills) (Variables|/Game/Blueprints/BP_Gun.BP_Gun_C|GetnotificationMessage (Variables|Default|GetGun))))))

(event Custom|AddKill
  (bind _result (Math|Integer|IncrementInt (Variables|Default|Getkills))
    (:%20%20
      (Variables|Default|Setkills _result)
      (Variables|/Game/Blueprints/BP_Gun.BP_Gun_C|SetnotificationMessage (Variables|Default|GetGun) "Nice!")
      (Default|UpdateHUD (Variables|Default|GetHUDReference) (Variables|/Game/Blueprints/BP_Gun.BP_Gun_C|GetcurrentBullets (Variables|Default|GetGun)) (Variables|Default|Getkills) (Variables|/Game/Blueprints/BP_Gun.BP_Gun_C|GetnotificationMessage (Variables|Default|GetGun))))))

(event Input|EnhancedActionEvents|EnhancedInputActionIA_Recargar
  (params (ActionValue :type Boolean) (ElapsedSeconds :type Float%20%28double-precision%29) (TriggeredSeconds :type Float%20%28double-precision%29) (InputAction :type Input%20Action%20Object%20Reference :default "/Game/Input/IA_Recargar.IA_Recargar"))
  (:Started
    (if (Variables|Default|GetisArmed)
      (Default|Reload (Variables|Default|GetGun))
      (Default|UpdateHUD (Variables|Default|GetHUDReference) (Variables|/Game/Blueprints/BP_Gun.BP_Gun_C|GetcurrentBullets (Variables|Default|GetGun)) (Variables|Default|Getkills) (Variables|/Game/Blueprints/BP_Gun.BP_Gun_C|GetnotificationMessage (Variables|Default|GetGun))))))

(event Input|EnhancedActionEvents|EnhancedInputActionIA_Disparar
  (params (ActionValue :type Boolean) (ElapsedSeconds :type Float%20%28double-precision%29) (TriggeredSeconds :type Float%20%28double-precision%29) (InputAction :type Input%20Action%20Object%20Reference :default "/Game/Input/IA_Disparar.IA_Disparar"))
  (:Started
    (if (Variables|Default|GetisArmed)
      (Default|Shoot (Variables|Default|GetGun))
      (Default|UpdateHUD (Variables|Default|GetHUDReference) (Variables|/Game/Blueprints/BP_Gun.BP_Gun_C|GetcurrentBullets (Variables|Default|GetGun)) (Variables|Default|Getkills) (Variables|/Game/Blueprints/BP_Gun.BP_Gun_C|GetnotificationMessage (Variables|Default|GetGun))))))

(event EventBeginPlay
  (Input|AddMappingContext (PlayerController|LocalPlayerSubsystems|GetEnhancedInputLocalPlayerSubsystem (Game|GetPlayerController 0)) "/Game/Input/IMC_Controls.IMC_Controls" 0 "(bIgnoreAllPressedKeysUntilRelease=True,bForceImmediately=False,bNotifyUserSettings=False)")
  (Utilities|FlowControl|Delay 1.0)
  ;[0.15 0.15 0.15 0.5] GuardarReferenciaHUD
  (bind _returnvalue (Actor|GetActorOfClass "/Game/Blueprints/BP_WidgetGameInfo.BP_WidgetGameInfo_C"))
  (bind _aswbp_game_info (Utilities|Casting|CastToWBP_GameInfo (UserInterface|GetUserWidgetObject (Variables|/Game/Blueprints/BP_WidgetGameInfo.BP_WidgetGameInfo_C|GetWidget _returnvalue))))
  (Variables|Default|SetHUDReference _aswbp_game_info))

(event Collision|EventActorBeginOverlap
  (params (OtherActor :type Actor%20Object%20Reference)))

(event EventTick
  (params (DeltaSeconds :type Float%20%28single-precision%29)))

(fn ConstructionScript)