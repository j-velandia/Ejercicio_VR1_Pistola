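; BP_Gun is a gun that fires BP_Bullet actors from a limited ammo count.
; BeginPlay fills CurrentBullets from DefaultQuantityBullets, and Shoot spends a round to spawn a bullet at the Arrow component's world transform.
; Reload raises the count to ReloadBullets when it is below that amount.
; Shoot and Reload write status text to NotificationMessage for rounds left, an empty gun or a successful reload.
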(event Custom|Shoot
  (if (> (Variables|Default|GetcurrentBullets) 0)
    (bind _result (Math|Integer|DecrementInt (Variables|Default|GetcurrentBullets))
      (:%20%20
        (Variables|Default|SetcurrentBullets _result)
        (Game|SpawnActorfromClass "/Game/Blueprints/BP_Bullet.BP_Bullet_C" (Transformation|GetWorldTransform (Variables|Default|GetArrow)) "Undefined" "MultiplyWithRoot" 0 0)
        (if (== (Variables|Default|GetcurrentBullets) 0)
          (Variables|Default|SetnotificationMessage "Out of ammo, reload!")
          (else
            (Variables|Default|SetnotificationMessage (Utilities|Text|FormatText "You have {bullets} rounds left" (Utilities|Text|ToText(Integer) (Variables|Default|GetcurrentBullets))))))))
    (else
      (Variables|Default|SetnotificationMessage "Reload! Press 'U' mf!!!"))))

(event Custom|Reload
  (if (< (Variables|Default|GetcurrentBullets) (Variables|Default|GetreloadBullets))
    (Variables|Default|SetcurrentBullets (Variables|Default|GetreloadBullets))
    (Variables|Default|SetnotificationMessage "Fire again!!")))

(event EventBeginPlay
  (Variables|Default|SetcurrentBullets (Variables|Default|GetdefaultQuantityBullets)))

(event Collision|EventActorBeginOverlap
  (params (OtherActor :type Actor%20Object%20Reference)))

(event EventTick
  (params (DeltaSeconds :type Float%20%28single-precision%29)))

(fn ConstructionScript)